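; BP_FixedCam is a fixed camera actor that runs an automated GPU performance capture.
; On BeginPlay it becomes the player's view target, then uses console commands to pin scalability, material quality, resolution and screen percentage, with VSync off and the frame rate uncapped.
; After short settling delays it records a timed CSV profile with GPU stats, then quits the game.
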(event `self.ReceiveBeginPlay`
  (`PlayerController.SetViewTargetWithBlend` (`GameplayStatics.GetPlayerController` 0) self 0.0 "VTBlend_Linear" 0.0 false)
  (`KismetSystemLibrary.Delay` 2.0)
  (`KismetSystemLibrary.ExecuteConsoleCommand` "scalability 3" null)
  (`KismetSystemLibrary.ExecuteConsoleCommand` "r.MaterialQualityLevel 1" null)
  (`KismetSystemLibrary.ExecuteConsoleCommand` "r.Vsync 0" null)
  (`KismetSystemLibrary.ExecuteConsoleCommand` "r.SetRes 1920x1080" null)
  (`KismetSystemLibrary.ExecuteConsoleCommand` "r.ScreenPercentage 100" null)
  (`KismetSystemLibrary.ExecuteConsoleCommand` "t.MaxFPS 0" null)
  (`KismetSystemLibrary.Delay` 3.0)
  (`KismetSystemLibrary.ExecuteConsoleCommand` "csvprofile start -csvGpuStats" null)
  (`KismetSystemLibrary.Delay` 30.0)
  (`KismetSystemLibrary.ExecuteConsoleCommand` "csvprofile stop" null)
  (`KismetSystemLibrary.Delay` 1.0)
  (`KismetSystemLibrary.QuitGame` null "Quit"))

(event `self.ReceiveTick`
  (params (DeltaSeconds :type "Float (single-precision)")))

(fn `UserConstructionScript`)